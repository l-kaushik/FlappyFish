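; Player pawn for a Flappy Bird-style game: a physics-driven fish that hops on touch or left click.
; Each press resets capsule velocities, then applies lift, spin and sound, while Tick applies corrective impulses against rising and positive pitch.
; A hit disables input-driven movement, shows the dead flipbook, then after a delay saves any high score and pauses on the game-over widget.
; BeginPlay loads or creates the save and adds the HUD.
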(event `self.ReceiveTick`
  (params (DeltaSeconds :type "Float (single-precision)"))
  (bind (_returnvalue_roll _returnvalue_pitch) (`KismetMathLibrary.BreakRotator` (`SceneComponent.K2_GetComponentRotation` (`self.Capsule`))))
  (`|ExecutionSequence`
    (:`then_0`
      (bind _returnvalue (`PrimitiveComponent.GetPhysicsLinearVelocity` (`self.Capsule`) "None"))
      (if (> (.z _returnvalue) 0.0)
        (`PrimitiveComponent.AddImpulse` (`self.Capsule`) (0.0 0.0 -15.0) "None" false)))
    (:`then_1`
      (if (> _returnvalue_pitch 0.0)
        (`PrimitiveComponent.AddAngularImpulseInDegrees` (`self.Capsule`) (0.0 500.0 0.0) "None" false)))))

(event `Key|Touch1`
  (params (Key :type "Key Structure"))
  (bind _capsule (`self.Capsule`))
  (:`Pressed`
    (if (`self.CanMove?`) :!label _label
      (`PrimitiveComponent.SetPhysicsLinearVelocity` _capsule (0.0 0.0 0.0) false "None")
      (`PrimitiveComponent.SetPhysicsAngularVelocityInDegrees` _capsule (0.0 0.0 0.0) false "None")
      (`PrimitiveComponent.AddImpulse` _capsule (0.0 0.0 550.0) "None" false)
      (`PrimitiveComponent.AddAngularImpulseInDegrees` _capsule (0.0 -10000.0 0.0) "None" false)
      (`GameplayStatics.PlaySoundAtLocation` "/Game/Assets/SFX/mixkit-arcade-game-jump-coin-216.mixkit-arcade-game-jump-coin-216" (`self.K2_GetActorLocation`) (struct) 1.0 1.0 0.0 null null null null))))

(event `Key|LeftMouseButton`
  (params (Key :type "Key Structure"))
  (:`Pressed`
    (goto _label)))

(event `self.ReceiveHit`
  (params (MyComp :type "PrimitiveComponent Object Reference") (Other :type "Actor Object Reference") (OtherComp :type "PrimitiveComponent Object Reference") (bSelfMoved :type Boolean) (HitLocation :type "Vector Structure") (HitNormal :type "Vector Structure") (NormalImpulse :type "Vector Structure") (Hit :type "HitResult Structure (by ref)"))
  (bind _score (`self.Score`))
  (bind _savegameref (`self.SaveGameRef`))
  (set `self.CanMove?` false)
  (`PaperFlipbookComponent.SetFlipbook` (`self.Player`) "/Game/Assets/Character/FishDead.FishDead")
  (`PrimitiveComponent.SetConstraintMode` (`self.Capsule`) "XZPlane")
  (`KismetSystemLibrary.Delay` 1.0)
  (if (> _score (`/Game/Blueprints/BP_SaveGame.SaveScore` _savegameref))
    (set `/Game/Blueprints/BP_SaveGame.SaveScore` _score _savegameref)
    (`GameplayStatics.SaveGameToSlot` _savegameref "1"))
  (bind _returnvalue (`|CreateWidget` "/Game/Blueprints/WB_GameOver.WB_GameOver_C"))
  (bind _output_get (set `self.GamveOverHUD` _returnvalue))
  (`TextBlock.SetText` (`/Game/Blueprints/WB_GameOver.PlayerScore` _output_get) (`KismetTextLibrary.Conv_IntToText` (`self.Score`)))
  (`TextBlock.SetText` (`/Game/Blueprints/WB_GameOver.PlayerHighScore` _output_get) (`KismetTextLibrary.Conv_IntToText` (`/Game/Blueprints/BP_SaveGame.SaveScore` (`self.SaveGameRef`))))
  (`UserWidget.AddToViewport` (`self.GamveOverHUD`) 0)
  (`GameplayStatics.SetGamePaused` true))

(event `IncreaseScore`
  (`/Engine/EditorBlueprintResources/StandardMacros.IncrementInt` (`self.Score`)))

(event `self.ReceiveBeginPlay`
  (bind _returnvalue (`GameplayStatics.GetPlayerController` 0))
  (set `PlayerController.bShowMouseCursor` false _returnvalue)
  (`WidgetBlueprintLibrary.SetInputMode_GameOnly` _returnvalue)
  (bind _returnvalue_2 (`GameplayStatics.DoesSaveGameExist` "1"))
  (if _returnvalue_2
    (bind _returnvalue_3 (`GameplayStatics.LoadGameFromSlot` "1"))
    (bind _asbp_save_game (cast `/Game/Blueprints/BP_SaveGame` _returnvalue_3))
    (set `self.SaveGameRef` _asbp_save_game)
    (else
      (bind _returnvalue_4 (`GameplayStatics.CreateSaveGameObject` "/Game/Blueprints/BP_SaveGame.BP_SaveGame_C"))
      (bind _output_get (set `self.SaveGameRef` _returnvalue_4))
      (`GameplayStatics.SaveGameToSlot` _output_get "1")))
  (bind _returnvalue_5 (`|CreateWidget` "/Game/Blueprints/WB_HUD.WB_HUD_C" null self))
  (bind _output_get_2 (set `self.PlayerHUD` _returnvalue_5))
  (`UserWidget.AddToViewport` _output_get_2 0))

(fn `UserConstructionScript`)